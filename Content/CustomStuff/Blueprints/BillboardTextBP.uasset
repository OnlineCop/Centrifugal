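; Billboard text actor that shows a separate copy of its text to each player, rotated to face that player's camera.
; BeginPlay spawns one text actor per PlayerController, owned by its pawn and set Only Owner See, and maps it to that camera manager.
; InitializeChildren copies the template TextRender's text, material, font and formatting onto each copy.
; Tick turns every copy toward its mapped camera's location.
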(event EventTick
  (params (DeltaSeconds :type Float%20%28single-precision%29))
  (bind _positions (Variables|Default|GetPositions))
  ;[1 1 1] Every TextRender must rotate toward its own look-at position
  (bind _keys (Utilities|Map|Keys _positions))
  (for _array_element _keys
    (if (.ReturnValue (Utilities|Map|Find _positions _array_element))
      (Transformation|SetWorldRotation (Variables|/Script/Engine.TextRenderActor|GetTextRender (.Value (Utilities|Map|Find _positions _array_element))) (Math|Rotator|FindLookatRotation (Transformation|GetWorldLocation (Variables|/Script/Engine.TextRenderActor|GetTextRender (.Value (Utilities|Map|Find _positions _array_element)))) (Camera|GetCameraLocation _array_element)) false false))))

(event EventBeginPlay
  ;[1 1 1] The number of players is dynamic: create a TextRender for each player, set the player as the TextRender's owner, and set Only Owner See.
  (bind _outactors (Actor|GetAllActorsOfClass "/Script/Engine.PlayerController"))
  (for _array_element _outactors
    (bind _returnvalue (Game|SpawnActorfromClass (Variables|Default|GetText%20Class) (Transformation|GetActorTransform) "AlwaysSpawn" (Pawn|GetControlledPawn _array_element) 0))
    (Utilities|Map|Add (Variables|Default|GetPositions) (Variables|/Script/Engine.PlayerController|GetPlayerCameraManager _array_element) _returnvalue)
    (DynamicChildren|InitializeChildren _returnvalue)))

(fn ConstructionScript)

(fn InitializeChildren
  (params (TextRenderActorReference :type Text%20Render%20Actor%20Object%20Reference))
  (bind _textrender (Variables|/Script/Engine.TextRenderActor|GetTextRender TextRenderActorReference))
  (Rendering|SetOnlyOwnerSee _textrender true :!class /Script/Engine.PrimitiveComponent)
  (Rendering|Components|TextRender|SetText _textrender (Variables|/Script/Engine.TextRenderComponent|GetText (Variables|Default|GetTextRender)))
  (Class|TextRenderComponent|SetTextMaterial _textrender (Variables|/Script/Engine.TextRenderComponent|GetTextMaterial (Variables|Default|GetTextRender)))
  (Class|TextRenderComponent|SetFont _textrender (Variables|/Script/Engine.TextRenderComponent|GetFont (Variables|Default|GetTextRender)))
  (Rendering|Components|TextRender|SetHorizontalAlignment _textrender (Variables|/Script/Engine.TextRenderComponent|GetHorizontalAlignment (Variables|Default|GetTextRender)))
  (Class|TextRenderComponent|SetVerticalAlignment _textrender (Variables|/Script/Engine.TextRenderComponent|GetVerticalAlignment (Variables|Default|GetTextRender)))
  (Rendering|Components|TextRender|SetTextRenderColor _textrender (Variables|/Script/Engine.TextRenderComponent|GetTextRenderColor (Variables|Default|GetTextRender)))
  (Rendering|Components|TextRender|SetXScale _textrender (Variables|/Script/Engine.TextRenderComponent|GetXScale (Variables|Default|GetTextRender)))
  (Rendering|Components|TextRender|SetYScale _textrender (Variables|/Script/Engine.TextRenderComponent|GetYScale (Variables|Default|GetTextRender)))
  (Rendering|Components|TextRender|SetWorldSize _textrender (Variables|/Script/Engine.TextRenderComponent|GetWorldSize (Variables|Default|GetTextRender)))
  (Class|TextRenderComponent|SetHorizSpacingAdjust _textrender (Variables|/Script/Engine.TextRenderComponent|GetHorizSpacingAdjust (Variables|Default|GetTextRender)))
  (Class|TextRenderComponent|SetVertSpacingAdjust _textrender (Variables|/Script/Engine.TextRenderComponent|GetVertSpacingAdjust (Variables|Default|GetTextRender))))