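; ZeroGravityBP is a placeable volume that switches off gravity for actors inside it.
; On begin overlap, actors tagged "Antigrav" get gravity disabled on their primitive root component, and on end overlap it is re-enabled.
; The construction script feeds the box extent into the Field particle system as random spawn bounds and sets particle density from average actor scale, keeping the effect's world scale at one.
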(event Collision|EventActorBeginOverlap
  (params (OtherActor :type Actor%20Object%20Reference))
  (if (Actor|ActorHasTag OtherActor "Antigrav")
    (bind _asprimitive_component (Utilities|Casting|CastToPrimitiveComponent (VehicleSound|GetRootComponent OtherActor)))
    (Physics|SetEnableGravity _asprimitive_component false)))

(event Collision|EventActorEndOverlap
  (params (OtherActor :type Actor%20Object%20Reference))
  (if (Actor|ActorHasTag OtherActor "Antigrav")
    (bind _asprimitive_component (Utilities|Casting|CastToPrimitiveComponent (VehicleSound|GetRootComponent OtherActor)))
    (Physics|SetEnableGravity _asprimitive_component true)))

(fn ConstructionScript
  (bind _returnvalue (Transformation|GetActorScale3D))
  (bind _field (Variables|Default|GetField))
  (bind _box (Variables|Default|GetBox))
  (bind (_x _y _z) (Math|Vector|BreakVector _returnvalue))
  (bind _returnvalue_2 (Components|Box|GetScaledBoxExtent _box))
  (bind _instanceparameters (Variables|/Script/Engine.ParticleSystemComponent|GetInstanceParameters _field))
  (Utilities|FlowControl|Sequence
    (:then_0
      (|SetBy-RefVar (Utilities|Array|Get(acopy) _instanceparameters) (Utilities|Struct|MakeParticleSysParam "Bounds" "PSPT_VectorRand" 0.0 0.0 _returnvalue_2 (Math|Vector|NegateVector _returnvalue_2)))
      (Transformation|SetWorldScale3D (Variables|Default|GetField) "1.000000,1.000000,1.000000"))
    (:then_1
      (|SetBy-RefVar (Utilities|Array|Get(acopy) _instanceparameters 1) (Utilities|Struct|MakeParticleSysParam "Particle Density" "PSPT_Scalar" (/ (+ (+ _x _y) _z) 3.0))))))